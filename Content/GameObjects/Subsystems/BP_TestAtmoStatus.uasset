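; Debug actor that displays the local atmosphere composition at its own location in the world.
; On BeginPlay it starts a looping 0.1-second timer.
; Each tick of the timer queries the Atmo subsystem for the status at the actor's position and writes the O2, CO2, N2 and Toxin values to its TextRender component.
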(event Custom|CheckStatus
  (bind _returnvalue (Transformation|GetActorLocation))
  (bind _atmo (Variables|Default|GetAtmo))
  (bind _returnvalue_2 (Class|WorldGrid|GetAtmoStatusbyLocation _atmo _returnvalue))
  (Rendering|Components|TextRender|SetText (Variables|Default|GetTextRender) (Utilities|Text|FormatText "O2: {O2} 
CO2: {CO2} 
N2: {N2} 
Toxin: {Toxin}" (Utilities|Text|ToText(Float) (.o2 _returnvalue_2) "HalfToEven" true 1 10 0 1) (Utilities|Text|ToText(Float) (.co2 _returnvalue_2) "HalfToEven" true 1 10 0 1) (Utilities|Text|ToText(Float) (.n2 _returnvalue_2) "HalfToEven" true 1 10 0 1) (Utilities|Text|ToText(Float) (.toxin _returnvalue_2) "HalfToEven" true 1 10 0 1))))

(event EventBeginPlay
  (Utilities|Time|SetTimerbyEvent (delegate Custom|CheckStatus) 0.1 true))

(fn ConstructionScript)