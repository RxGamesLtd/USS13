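; BP_WorldGrid is a world grid Blueprint that sizes a gridded cube and a ground box from its Size and CellExtent.
; The construction script creates a dynamic GridMat instance on the Cube and passes the cell's X extent to it as a scalar parameter.
; It scales the Cube in X and Y to Size times CellExtent, converted from units, and sets the Ground box extent from the same product.
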(fn ConstructionScript
  (bind _size (Variables|Default|GetSize))
  (bind _cellextent (Variables|Default|GetCellExtent))
  (bind _returnvalue (* _size _cellextent))
  (Utilities|FlowControl|Sequence
    (:then_0
      (bind _returnvalue_2 (Rendering|Material|CreateDynamicMaterialInstance (Variables|Default|GetCube) 0 "/Game/USS13/GameObjects/Subsystems/WorldGrid/GridMat.GridMat" :!class /Script/Engine.PrimitiveComponent))
      (bind _output_get (Variables|Default|SetGridMat _returnvalue_2))
      (Rendering|Material|SetScalarParameterValue _output_get "CellExtent" (.x (Variables|Default|GetCellExtent)) :!class /Script/Engine.MaterialInstanceDynamic))
    (:then_1
      (Transformation|SetRelativeScale3D (Variables|Default|GetCube) (/ (Math|Vector|MakeVector (.x _returnvalue) (.y _returnvalue) 1.0) 50)))
    (:then_2
      (Components|Box|SetBoxExtent (Variables|Default|GetGround) (* (Variables|Default|GetSize) (Variables|Default|GetCellExtent)) true))))