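; Fog of war subsystem actor that renders the fog through a post-process material.
; The construction script creates a dynamic instance of the fog material and adds it as a PostProcess blendable.
; On each fog texture update, it passes current and previous textures to the material and resets the blend.
; Tick then crossfades between them over about a tenth of a second and flags IsDoneBlending once complete.
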(event EventTick
  (params (DeltaSeconds :type Float%20%28single-precision%29))
  (if (< (Variables|Default|GetFOWTextureBlend) 1.0)
    (bind _output_get (Variables|Default|SetFOWTextureBlend (Math|Float|Clamp(Float) (+ (* DeltaSeconds 1e+01) (Variables|Default|GetFOWTextureBlend)))))
    (Rendering|Material|SetScalarParameterValue (Variables|Default|GetDinamicMat) "Blend" _output_get :!class /Script/Engine.MaterialInstanceDynamic)
    (elif (not (Variables|Default|GetbIsDoneBlending))
      (Variables|Default|SetbIsDoneBlending true))))

(event EventOnFowTextureUpdated
  (params (currentTexture :type Texture%202D%20Object%20Reference) (lastTexture :type Texture%202D%20Object%20Reference))
  (bind _dinamicmat (Variables|Default|GetDinamicMat))
  (Rendering|Material|SetTextureParameterValue _dinamicmat "FOWTexture" currentTexture)
  (Rendering|Material|SetTextureParameterValue _dinamicmat "LastFOWTexture" lastTexture)
  (Rendering|Material|SetScalarParameterValue _dinamicmat "Blend" 0.0 :!class /Script/Engine.MaterialInstanceDynamic)
  (Variables|Default|SetFOWTextureBlend 0.0))

(fn ConstructionScript
  (bind _returnvalue (Rendering|Material|CreateDynamicMaterialInstance "/Game/USS13/GameObjects/Subsystems/FogOfWar/FOWMat.FOWMat" :!class /Script/Engine.KismetMaterialLibrary))
  (bind _output_get (Variables|Default|SetDinamicMat _returnvalue))
  (Rendering|AddorUpdateBlendable (Variables|Default|GetPostProcess) _output_get 1.0 :!class /Script/Engine.PostProcessComponent))