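; Player controller that drives a Mannequin pawn with camera-yaw-relative axis input and provides grid-based floor and wall building.
; T cycles Moving, Floor and Wall modes; Tick traces under the cursor, snaps the build location and previews it with a debug box.
; Walls snap to the nearer of two candidate cell edges, setting their orientation, and clicking spawns the piece.
; R registers the pawn with fog-of-war actors for debugging; old click-to-move logic is disconnected.
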(event EventTick
  (params (DeltaSeconds :type Float%20%28single-precision%29))
  (bind _cellsize (Variables|Default|GetCellSize))
  (bind _cellsize_2 (Variables|Default|GetCellSize))
  (bind _cellsize_3 (Variables|Default|GetCellSize))
  (bind _cellsize_4 (Variables|Default|GetCellSize))
  (bind _cellsize_5 (Variables|Default|GetCellSize))
  (bind _returnvalue (/ _cellsize 2.0))
  (bind _returnvalue_2 (/ _cellsize_4 2.0))
  (bind _returnvalue_3 (/ _cellsize_5 2.0))
  (bind _returnvalue_4 (Math|Vector|MakeVector 1e+01 _returnvalue_2 1e+02))
  (Variables|Default|SetMouseFloorHIt (.impactpoint (.HitResult (Game|Player|GetHitResultUnderCursorbyChannel "TraceTypeQuery3" true))))
  (switch Utilities|FlowControl|Switch|SwitchonConstructMode (Variables|Default|GetbConstructMode)
    (:NewEnumerator1
      (Utilities|FlowControl|Sequence
        (:then_0
          (Variables|Default|SetBuildBoxLocation (Math|Vector|MakeVector (CallFunction|SpanGridOffset (.X (Math|Vector|BreakVector (Variables|Default|GetMouseFloorHIt))) _cellsize _returnvalue) (CallFunction|SpanGridOffset (.Y (Math|Vector|BreakVector (Variables|Default|GetMouseFloorHIt))) _cellsize _returnvalue) 0.0)))
        (:then_1
          (Rendering|Debug|DrawDebugBox (Variables|Default|GetBuildBoxLocation) (Math|Vector|MakeVector _returnvalue_3 _returnvalue_3 1e+01) "(R=1.000000,G=0.000000,B=0.398461,A=1.000000)" "0, 0, 0" 0.0 0.0))))
    (:NewEnumerator2
      (Utilities|FlowControl|Sequence
        (:then_0
          (Variables|Default|SetDebugBoxLocRight (Math|Vector|MakeVector (CallFunction|SpanGridOffset (.X (Math|Vector|BreakVector (Variables|Default|GetMouseFloorHIt))) _cellsize_3 (/ _cellsize_3 -2.0)) (CallFunction|SpanGridOffset (.Y (Math|Vector|BreakVector (Variables|Default|GetMouseFloorHIt))) _cellsize_3 0.0) 0.0)))
        (:then_1
          (Variables|Default|SetDebugBoxLocFront (Math|Vector|MakeVector (CallFunction|SpanGridOffset (.X (Math|Vector|BreakVector (Variables|Default|GetMouseFloorHIt))) _cellsize_2 0.0) (CallFunction|SpanGridOffset (.Y (Math|Vector|BreakVector (Variables|Default|GetMouseFloorHIt))) _cellsize_2 (/ _cellsize_2 -2.0)) 0.0)))
        (:then_2
          (Math|Float|CompareFloat (Math|Vector|VectorLengthSquared (- (Variables|Default|GetDebugBoxLocRight) (Variables|Default|GetMouseFloorHIt))) (Math|Vector|VectorLengthSquared (- (Variables|Default|GetMouseFloorHIt) (Variables|Default|GetDebugBoxLocFront)))
            (:>
              (Variables|Default|SetBuildBoxLocation (Variables|Default|GetDebugBoxLocFront) :!label _label)
              (Variables|Default|SetWallFront true))
            (:==
              (goto _label))
            (:<
              (Variables|Default|SetBuildBoxLocation (Variables|Default|GetDebugBoxLocRight))
              (Variables|Default|SetWallFront false))))
        (:then_3
          (if (Variables|Default|GetWallFront)
            (Rendering|Debug|DrawDebugBox (+ (Variables|Default|GetBuildBoxLocation) "0, 0,100.000000") _returnvalue_4 "(R=0.000000,G=1.000000,B=0.038660,A=1.000000)" "0, 0, 0" 0.0 0.0)
            (else
              (Rendering|Debug|DrawDebugBox (+ (Variables|Default|GetBuildBoxLocation) "0, 0,100.000000") _returnvalue_4 "(R=1.000000,G=0.000000,B=0.398461,A=1.000000)" "0,90.000000, 0" 0.0 0.0))))))))

(event Input|ActionEvents|InputActionSetDestination
  (params (Key :type Key%20Structure :default "AnyKey"))
  (:Pressed
    (Variables|Default|SetbMoveToCursor true)
    (switch Utilities|FlowControl|Switch|SwitchonConstructMode (Variables|Default|GetbConstructMode)
      (:NewEnumerator1
        (Game|SpawnActorfromClass "/Game/USS13/GameObjects/Structures/BP_FloorBase.BP_FloorBase_C" (Math|Transform|MakeTransform (Variables|Default|GetBuildBoxLocation)) "Undefined" 0 0))
      (:NewEnumerator2
        (if (Variables|Default|GetWallFront)
          (Game|SpawnActorfromClass "/Game/USS13/GameObjects/Structures/BP_WallBase.BP_WallBase_C" (Math|Transform|MakeTransform (Variables|Default|GetBuildBoxLocation) "0.000000,90.000000, 0") "Undefined" 0 0)
          (else
            (Game|SpawnActorfromClass "/Game/USS13/GameObjects/Structures/BP_WallBase.BP_WallBase_C" (Math|Transform|MakeTransform (Variables|Default|GetBuildBoxLocation)) "Undefined" 0 0))))))
  (:Released
    (Variables|Default|SetbMoveToCursor false)))

(event Input|AxisEvents|InputAxisMoveForward
  (params (AxisValue :type Float%20%28single-precision%29))
  ;[1 1 1] Movement
  (bind _asmannequin (Utilities|Casting|CastToMannequin (Pawn|GetControlledPawn)))
  (Pawn|Input|AddMovementInput _asmannequin (Math|Vector|GetForwardVector (Math|Rotator|MakeRotator 0.0 0.0 (.yaw (Camera|GetCameraRotation (Game|GetPlayerCameraManager 0))))) AxisValue false))

(event Input|AxisEvents|InputAxisMoveRight
  (params (AxisValue :type Float%20%28single-precision%29))
  ;[1 1 1] Movement
  (bind _asmannequin (Utilities|Casting|CastToMannequin (Pawn|GetControlledPawn)))
  (Pawn|Input|AddMovementInput _asmannequin (Math|Vector|GetRightVector (Math|Rotator|MakeRotator 0.0 0.0 (.yaw (Camera|GetCameraRotation (Game|GetPlayerCameraManager 0))))) AxisValue false))

(event Input|KeyboardEvents|T
  (params (Key :type Key%20Structure :default "AnyKey"))
  (:Pressed
    (switch Utilities|FlowControl|Switch|SwitchonConstructMode (Variables|Default|GetbConstructMode)
      (:NewEnumerator0
        (Variables|Default|SetbConstructMode "NewEnumerator1"))
      (:NewEnumerator1
        (Variables|Default|SetbConstructMode "NewEnumerator2"))
      (:NewEnumerator2
        (Variables|Default|SetbConstructMode "NewEnumerator0")))))

(event Input|KeyboardEvents|R
  (params (Key :type Key%20Structure :default "AnyKey"))
  ;[1 1 1] Debug register pawn
  (:Released
    (bind _outactors (Actor|GetAllActorsOfClass "/Game/USS13/GameObjects/Subsystems/BP_PlanarFOW.BP_PlanarFOW_C"))
    (for _array_element _outactors
      (Class|FogPlane|RegisterFowActor _array_element (Pawn|GetControlledPawn)))))

(fn ConstructionScript)