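; Top-down player controller with grid-based building, where T cycles between Moving, Floor and Wall modes.
; Tick traces under the cursor, snaps the point to an offset grid and previews it with debug boxes, choosing wall orientation from the nearer of two candidates.
; SetDestination spawns a floor or wall there.
; Axis inputs move the TopDownCharacter relative to camera yaw; the old click-to-move logic is disconnected.
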(event EventTick
  (params (DeltaSeconds :type Float%20%28single-precision%29))
  (Variables|Default|SetMouseFloorHIt (.impactpoint (.HitResult (Game|Player|GetHitResultUnderCursorbyChannel "TraceTypeQuery3" true))))
  (switch Utilities|FlowControl|Switch|SwitchonConstructMode (Variables|Default|GetbConstructMode)
    (:NewEnumerator1
      (Utilities|FlowControl|Sequence
        (:then_0
          (Variables|Default|SetBuildBoxLocation (Math|Vector|MakeVector (CallFunction|SpanGridOffset (.X (Math|Vector|BreakVector (Variables|Default|GetMouseFloorHIt))) 1.5e+02 75.0) (CallFunction|SpanGridOffset (.Y (Math|Vector|BreakVector (Variables|Default|GetMouseFloorHIt))) 1.5e+02 75.0) 0.0)))
        (:then_1
          (Rendering|Debug|DrawDebugBox (Variables|Default|GetBuildBoxLocation) "75.000000,75.000000,10.000000" "(R=1.000000,G=0.000000,B=0.398461,A=1.000000)" "0, 0, 0" 0.0))))
    (:NewEnumerator2
      (Utilities|FlowControl|Sequence
        (:then_0
          (Variables|Default|SetDebugBoxLocRight (Math|Vector|MakeVector (CallFunction|SpanGridOffset (.X (Math|Vector|BreakVector (Variables|Default|GetMouseFloorHIt))) 1.5e+02 -75.0) (CallFunction|SpanGridOffset (.Y (Math|Vector|BreakVector (Variables|Default|GetMouseFloorHIt))) 1.5e+02 0.0) 0.0)))
        (:then_1
          (Variables|Default|SetDebugBoxLocFront (Math|Vector|MakeVector (CallFunction|SpanGridOffset (.X (Math|Vector|BreakVector (Variables|Default|GetMouseFloorHIt))) 1.5e+02 0.0) (CallFunction|SpanGridOffset (.Y (Math|Vector|BreakVector (Variables|Default|GetMouseFloorHIt))) 1.5e+02 -75.0) 0.0)))
        (:then_2
          (Math|Float|CompareFloat (Math|Vector|VectorLengthSquared (- (Variables|Default|GetDebugBoxLocRight) (Variables|Default|GetMouseFloorHIt))) (Math|Vector|VectorLengthSquared (- (Variables|Default|GetMouseFloorHIt) (Variables|Default|GetDebugBoxLocFront)))
            (:>
              (Variables|Default|SetBuildBoxLocation (Variables|Default|GetDebugBoxLocFront) :!label _label)
              (Variables|Default|SetWallFront true))
            (:==
              (goto _label))
            (:<
              (Variables|Default|SetBuildBoxLocation (Variables|Default|GetDebugBoxLocRight))
              (Variables|Default|SetWallFront false))))
        (:then_3
          (if (Variables|Default|GetWallFront)
            (Rendering|Debug|DrawDebugBox (+ (Variables|Default|GetBuildBoxLocation) "0, 0,100.000000") "10.000000,75.000000,100.000000" "(R=0.000000,G=1.000000,B=0.038660,A=1.000000)" "0, 0, 0" 0.0)
            (else
              (Rendering|Debug|DrawDebugBox (+ (Variables|Default|GetBuildBoxLocation) "0, 0,100.000000") "75.000000,10.000000,100.000000" "(R=1.000000,G=0.000000,B=0.398461,A=1.000000)" "0, 0, 0" 0.0))))))))

(event Input|ActionEvents|InputActionSetDestination
  (params (Key :type Key%20Structure :default "AnyKey"))
  (:Pressed
    (Variables|Default|SetbMoveToCursor true)
    (switch Utilities|FlowControl|Switch|SwitchonConstructMode (Variables|Default|GetbConstructMode)
      (:NewEnumerator1
        (Game|SpawnActorfromClass "/Game/GameObjects/Structures/FloorBase.FloorBase_C" (Math|Transform|MakeTransform (Variables|Default|GetBuildBoxLocation) "0, 0, 0" "1.000000,1.000000,1.000000") "Undefined" 0 0))
      (:NewEnumerator2
        (if (Variables|Default|GetWallFront)
          (Game|SpawnActorfromClass "/Game/GameObjects/Structures/WallBase.WallBase_C" (Math|Transform|MakeTransform (Variables|Default|GetBuildBoxLocation) "0.000000,90.000000, 0" "1.000000,1.000000,1.000000") "Undefined" 0 0)
          (else
            (Game|SpawnActorfromClass "/Game/GameObjects/Structures/WallBase.WallBase_C" (Math|Transform|MakeTransform (Variables|Default|GetBuildBoxLocation) "0,0.000000, 0" "1.000000,1.000000,1.000000") "Undefined" 0 0))))))
  (:Released
    (Variables|Default|SetbMoveToCursor false)))

(event Input|AxisEvents|InputAxisMoveForward
  (params (AxisValue :type Float%20%28single-precision%29))
  ;[1 1 1] Movement
  (bind _astop_down_character (Utilities|Casting|CastToTopDownCharacter (Pawn|GetControlledPawn)))
  (Pawn|Input|AddMovementInput _astop_down_character (Math|Vector|GetForwardVector (Math|Rotator|MakeRotator 0.0 0.0 (.yaw (Camera|GetCameraRotation (Game|GetPlayerCameraManager 0))))) AxisValue false))

(event Input|AxisEvents|InputAxisMoveRight
  (params (AxisValue :type Float%20%28single-precision%29))
  ;[1 1 1] Movement
  (bind _astop_down_character (Utilities|Casting|CastToTopDownCharacter (Pawn|GetControlledPawn)))
  (Pawn|Input|AddMovementInput _astop_down_character (Math|Vector|GetRightVector (Math|Rotator|MakeRotator 0.0 0.0 (.yaw (Camera|GetCameraRotation (Game|GetPlayerCameraManager 0))))) AxisValue false))

(event Input|KeyboardEvents|T
  (params (Key :type Key%20Structure :default "AnyKey"))
  (:Pressed
    (switch Utilities|FlowControl|Switch|SwitchonConstructMode (Variables|Default|GetbConstructMode)
      (:NewEnumerator0
        (Variables|Default|SetbConstructMode "NewEnumerator1"))
      (:NewEnumerator1
        (Variables|Default|SetbConstructMode "NewEnumerator2"))
      (:NewEnumerator2
        (Variables|Default|SetbConstructMode "NewEnumerator0")))))

(fn ConstructionScript)